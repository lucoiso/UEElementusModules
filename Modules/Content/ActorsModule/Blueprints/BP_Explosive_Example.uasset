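; BP_Explosive_Example is an example actor that triggers an explosion through a child activator platform.
; On BeginPlay, only the authority binds CharacterStepUp to the platform's toggled-by-character event.
; That handler calls PerformExplosion and prints a message without checking IsBegin, so it does not distinguish between the two toggle states.
; The construction script labels the platform's text render as the explosive example.
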(event `self.ReceiveBeginPlay`
  (`/Engine/EditorBlueprintResources/ActorMacros.Switch Has Authority`
    (:`Authority`
      (bind _asbp_activator_platform (cast `/ElementusModules/CommonModule/Actors/BP_ActivatorPlatform` (`ChildActorComponent.ChildActor` (`self.Platform`))))
      (add `/ElementusModules/CommonModule/Actors/BP_ActivatorPlatform.ToggledByCharacter` _asbp_activator_platform (delegate `CharacterStepUp`)))))

(event `CharacterStepUp`
  (params (Character :type "PECharacter Object Reference") (IsBegin :type Boolean))
  (`self.PerformExplosion`)
  (`KismetSystemLibrary.PrintString` "Explosion Started"))

(fn `UserConstructionScript`
  (bind _asbp_activator_platform (cast `/ElementusModules/CommonModule/Actors/BP_ActivatorPlatform` (`ChildActorComponent.ChildActor` (`self.Platform`))))
  (`TextRenderComponent.K2_SetText` (`/ElementusModules/CommonModule/Actors/BP_ActivatorPlatform.TextRender` _asbp_activator_platform) "Explosive Example"))