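; Example actor that toggles a dynamic Enhanced Input binding on a player when their locally controlled PECharacter overlaps its capsule.
; The toggle binds a configurable action, trigger event and named function on a target object, then adds an input mapping, or removes both if already bound.
; PlayerBindingData stores the returned per-controller handles for lookup and removal.
; ExampleFunction is a print-only sample callback, and debug prints report each toggle.
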(event `self.Capsule.OnComponentBeginOverlap`
  (params (OverlappedComponent :type "PrimitiveComponent Object Reference") (OtherActor :type "Actor Object Reference") (OtherComp :type "PrimitiveComponent Object Reference") (OtherBodyIndex :type Integer) (bFromSweep :type Boolean) (SweepResult :type "HitResult Structure (by ref)"))
  (bind _aspecharacter (cast `PECharacter` OtherActor))
  (if (`Pawn.IsLocallyControlled` _aspecharacter)
    (bind _asplayer_controller (cast `PlayerController` (`Pawn.GetController` _aspecharacter)))
    (`self.ToggleDynamicActionAddition` _asplayer_controller)))

(event `ExampleFunction`
  ;[0 0 0] Example Function
  (`KismetSystemLibrary.PrintString` "Function Called"))

(event `ToggleDynamicActionAddition`
  (params (Controller :type "PlayerController Object Reference"))
  (bind (_bindinghandle _returnvalue) (`PEPlayerLibrary.CheckIfPlayerContainsDynamicInput` Controller (`self.PlayerBindingData`)))
  ;[0.06112 1 0] AddRemove Logic
  (if _returnvalue
    (`PEPlayerLibrary.RemoveDynamicInput` _bindinghandle)
    (`KismetArrayLibrary.Array_RemoveItem` (`self.PlayerBindingData`) _bindinghandle)
    (`PEPlayerLibrary.RemoveDynamicMapping` Controller (`self.InputMapping`))
    (`KismetSystemLibrary.PrintString` "Dynamic Bind Removed" true true (struct :`R` 1.0 :`A` 1.0))
    (else
      (bind _returnvalue_2 (`PEPlayerLibrary.BindDynamicInput` Controller (`self.InputAction`) (`self.FunctionOwner`) (`self.FunctionName`) (`self.TriggerEvent`)))
      (`KismetArrayLibrary.Array_Add` (`self.PlayerBindingData`) _returnvalue_2)
      (`PEPlayerLibrary.AddDynamicMapping` Controller (`self.InputMapping`) 1)
      (`KismetSystemLibrary.PrintString` "Dynamic Bind Added" true true (struct :`G` 1.0 :`A` 1.0))
      (`KismetSystemLibrary.PrintString` "Press F" true true (struct :`G` 1.0 :`A` 1.0)))))

(fn `CheckIfContainsPlayer`
  (params (Controller :type "PlayerController Object Reference"))
  (returns (Result :type Boolean) (FoundHandle :type "PlayerInputBindingHandle Structure"))
  (bind _playerbindingdata (`self.PlayerBindingData`))
  (if (`KismetArrayLibrary.Array_IsEmpty` _playerbindingdata)
    (return false)
    (else
      (for _array_element _playerbindingdata
        (bind _returnvalue (== (break `PlayerInputBindingHandle` _array_element) Controller))
        (if _returnvalue
          (break)))
      (return _returnvalue (make `PlayerInputBindingHandle` (break `PlayerInputBindingHandle` _array_element) (`.InputBindingHandle` (break `PlayerInputBindingHandle` _array_element)))))))

(fn `UserConstructionScript`)