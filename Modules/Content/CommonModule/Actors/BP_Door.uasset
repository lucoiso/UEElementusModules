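; Interactable door actor that swings open 90 degrees away from or toward a side chosen by the interacting character's position, then closes on the next interaction.
; A FlipFlop plays or reverses a timeline that lerps the DoorOffset rotation on authority only.
; Interaction is locked during the swing.
; Replication is switched on at interaction and off shortly after the timeline finishes.
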(event `PerformDoorRotation`
  ;[0 0 0] Performs the interaction behavior: in this case will rotate the door mesh
  (set `self.bIsInteractionEnabled` false)
  (bind _return (`self.GetRotationDirection`))
  (`/Engine/EditorBlueprintResources/StandardMacros.FlipFlop`
    (:`A`
      (bind (_direction _alpha) (`Timeline|DoorTimeline` :!label _label)
        (:`Update`
          (`/Engine/EditorBlueprintResources/ActorMacros.Switch Has Authority`
            (:`Authority`
              (`SceneComponent.K2_SetRelativeRotation` (`self.DoorOffset`) (`KismetMathLibrary.RLerp` (struct) _return _alpha) false false))))
        (:`Finished`
          (set `self.bIsInteractionEnabled` true)
          (`KismetSystemLibrary.Delay` 0.2)
          (`self.SetReplicates` (not (`self.bIsInteractionEnabled`))))))
    (:`B`
      (goto _label :!via `Reverse`))))

(event `self.DoInteractionBehavior`
  (params (CharacterInteracting :type "Character Object Reference") (HitResult :type "HitResult Structure (by ref)"))
  ;[0 1 0.02242] Initialize Interaction if Enabled
  (`/Engine/EditorBlueprintResources/StandardMacros.IsValid` CharacterInteracting
    (:`Is Valid`
      (if (`PEInteractable.IsInteractEnabled`)
        (set `self.LastRelativeInteractionLocation` (- (`self.K2_GetActorLocation` CharacterInteracting) (`SceneComponent.K2_GetComponentLocation` (`self.StaticMesh`))))
        (`self.SetReplicates` true)
        (`self.PerformDoorRotation`)))))

(fn `GetRotationDirection`
  (returns (Return :type "Rotator Structure"))
  (bind _relativerotation (`SceneComponent.RelativeRotation` (`self.DoorOffset`)))
  (bind (_returnvalue_x _returnvalue_y) (`KismetMathLibrary.BreakVector` (`KismetMathLibrary.GetDirectionUnitVector` (`SceneComponent.RelativeLocation` (`self.StaticMesh`)) (`self.LastRelativeInteractionLocation`))))
  (if (!= _relativerotation (struct))
    (return _relativerotation)
    (elif (< _returnvalue_y 0.0)
      (return (struct :`Yaw` 90.0))
      (else
        (return (struct :`Yaw` -90.0))))))

(fn `IsInteractEnabled`
  (returns (ReturnValue :type Boolean))
  (return (`self.bIsInteractionEnabled`)))

(fn `UserConstructionScript`)