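; Elevator actor whose platform travels between its origin and a final location reference, toggling direction each time its box is overlapped while idle.
; An overlap enables replication and fades the platform's dynamic material color on a timeline, then a FlipFlop plays or reverses the movement timeline, moving the platform only on authority.
; On finish it restores the color and, after a short delay, disables replication.
; The construction script zeroes both text labels' world rotation.
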(event `self.ReceiveBeginPlay`
  ;[0.04294 1 0] BeginPlay: Initialize Dynamic Material
  (bind _returnvalue (`PrimitiveComponent.CreateDynamicMaterialInstance` (`self.Platform`) 0 "/Game/Main/Materials/Instances/MI_Solid_Blue.MI_Solid_Blue" "None"))
  (set `self.Platform_MatRef` _returnvalue))

(event `Change Color`
  ;[0 0 0] Set Platform Material Color
  (if (`self.bIsMoving`)
    (bind (_direction _color) (`Timeline|Color Timeline` :!label _label)
      (:`Update`
        (`MaterialInstanceDynamic.SetVectorParameterValue` (`self.Platform_MatRef`) "Base Color" (`KismetMathLibrary.Conv_VectorToLinearColor` _color))))
    (else
      (goto _label :!via `Reverse`))))

(event `TogglePlatformMovement`
  ;[1 0.75 0] Movement Logic
  (`/Engine/EditorBlueprintResources/StandardMacros.FlipFlop`
    (:`A`
      (bind (_direction _alpha) (`Timeline|MovementTimeline` :!label _label_2)
        (:`Update`
          (`/Engine/EditorBlueprintResources/ActorMacros.Switch Has Authority`
            (:`Authority`
              (`SceneComponent.K2_SetRelativeLocation` (`self.Platform`) (`KismetMathLibrary.VLerp` (0.0 0.0 0.0) (`SceneComponent.RelativeLocation` (`self.Final_Location_Ref`)) _alpha) false false))))
        (:`Finished`
          (set `self.bIsMoving` false)
          (`self.Change Color`)
          (`KismetSystemLibrary.Delay` 0.2)
          (`self.SetReplicates` (`self.bIsMoving`)))))
    (:`B`
      (goto _label_2 :!via `Reverse`))))

(event `self.Box.OnComponentBeginOverlap`
  (params (OverlappedComponent :type "PrimitiveComponent Object Reference") (OtherActor :type "Actor Object Reference") (OtherComp :type "PrimitiveComponent Object Reference") (OtherBodyIndex :type Integer) (bFromSweep :type Boolean) (SweepResult :type "HitResult Structure (by ref)"))
  ;[0 0.2433 1] Detect Overlap
  (if (not (`self.bIsMoving`))
    (`self.SetReplicates` true)
    (set `self.bIsMoving` true)
    (`self.Change Color`)
    (`KismetSystemLibrary.Delay` (`TimelineComponent.GetTimelineLength` (`self.Color Timeline`)))
    (`self.TogglePlatformMovement`)))

(fn `UserConstructionScript`
  (`SceneComponent.K2_SetWorldRotation` :`self` (`self.Initial_Text`))
  (`SceneComponent.K2_SetWorldRotation` :`self` (`self.Final_Text`)))