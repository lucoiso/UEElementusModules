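; BP_Ability_Example is an example actor that toggles a configured gameplay ability on characters that overlap its capsule.
; The overlap runs only with authority and acts only on PECharacters, using their ability system component.
; It removes the ability if the character already has it, otherwise grants it bound to an InputID from EN_AbilityInputID, and prints a message either way.
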(event `self.Capsule.OnComponentBeginOverlap`
  (params (OverlappedComponent :type "PrimitiveComponent Object Reference") (OtherActor :type "Actor Object Reference") (OtherComp :type "PrimitiveComponent Object Reference") (OtherBodyIndex :type Integer) (bFromSweep :type Boolean) (SweepResult :type "HitResult Structure (by ref)"))
  (bind _gameplayability (`self.GameplayAbility`))
  (`/Engine/EditorBlueprintResources/ActorMacros.Switch Has Authority`
    (:`Authority`
      (bind _aspecharacter (cast `PECharacter` OtherActor))
      (bind _returnvalue (`AbilitySystemBlueprintLibrary.GetAbilitySystemComponent` _aspecharacter))
      (if (`PEAbilityFunctions.HasAbilityWithClass` _returnvalue _gameplayability)
        (`PEAbilityFunctions.RemoveAbility` _returnvalue _gameplayability)
        (`KismetSystemLibrary.PrintString` "Ability Removed" true true (struct :`R` 1.0 :`A` 1.0))
        (else
          (`PEAbilityFunctions.GiveAbility` _returnvalue _gameplayability (`self.InputID`) "/ElementusModules/AbilitySystemModule/Data/EN_AbilityInputID.EN_AbilityInputID" false true)
          (`KismetSystemLibrary.PrintString` "Ability Added" true true (struct :`G` 1.0 :`A` 1.0)))))))

(fn `UserConstructionScript`)